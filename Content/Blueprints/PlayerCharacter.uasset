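; Player helicopter character for a MASH-style rescue game: it picks up soldiers up to capacity, drops them at hospitals and triggers game over on hitting a tree.
; Axis inputs drive movement, and capsule hits cast the other actor to choose the outcome and sound.
; Tick advances a timer through a one-second Delay and recalculates score from rescued, held and time.
; Reset input destroys the level's actors and reloads it as a level instance.
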(event `self.ReceiveBeginPlay`
  ;[1 1 1] Background Game Music
  (`AudioComponent.Play` (`self.Background_Music`) 0.0))

(event `InputAxis|MoveRight`
  (params (AxisValue :type "Float (single-precision)"))
  ;[1 1 1] Adding Player Input
  (`self.AddMovementInput` (1.0 0.0 0.0) AxisValue))

(event `self.ReceiveTick`
  (params (DeltaSeconds :type "Float (single-precision)"))
  (`|ExecutionSequence`
    (:`then_0`
      ;[1 1 1] Setting up and updating the timer variables
      (`KismetSystemLibrary.Delay` 1.0)
      (set `self.Seconds` (+ (`self.Seconds`) 1))
      (if (> (`self.Seconds`) 59)
        (set `self.Minutes` (+ (`self.Minutes`) 1))
        (set `self.Seconds` 0)))
    (:`then_1`
      (`self.Calculate Score`))))

(event `InputAxis|MoveUp`
  (params (AxisValue :type "Float (single-precision)"))
  ;[1 1 1] Adding Player Input
  (`self.AddMovementInput` (0.0 -1.0 1.0) AxisValue))

(event `self.CapsuleComponent.OnComponentHit`
  (params (HitComponent :type "PrimitiveComponent Object Reference") (OtherActor :type "Actor Object Reference") (OtherComp :type "PrimitiveComponent Object Reference") (NormalImpulse :type "Vector Structure") (Hit :type "HitResult Structure (by ref)"))
  ;[1 1 1] Logic for Helicopter Collisions with other Actors
  ;;[1 1 1] If Hit Soldier, DestroyActor and Holding++
  (bind _assoldier_character (cast `/Game/Blueprints/SoldierCharacter` OtherActor)
    (:`then`
      ;;[1 1 1] Check if the Helicopter has enough Capacity
      (if (< (`self.Holding`) (`self.Helicopter Capacity`))
        (`self.K2_DestroyActor` _assoldier_character)
        (`GameplayStatics.PlaySound2D` "/Game/Sounds/Pickup_Sound2_Cue.Pickup_Sound2_Cue" 1.0 1.0 0.0 null null)
        ;;[1 1 1] Adding hit soldier to "Holding" and Updating the UI widget
        (set `self.Holding` (+ (`self.Holding`) 1))
        (bind _asmash_hud (cast `/Game/Blueprints/Mash_HUD` (`PlayerController.GetHUD` (`GameplayStatics.GetPlayerController` 0))))
        (else
          (`GameplayStatics.PlaySound2D` "/Game/Sounds/Disappointed/8bit_Error.8bit_Error" 1.0 1.0 0.0 "/Game/Sounds/Error_Concurrency.Error_Concurrency" null))))
    (:`CastFailed`
      ;;[1 1 1] If Hit Hospital
      (cast `/Game/Blueprints/Hospital` OtherActor
        (:`then`
          ;;[1 1 1] If Holding > 0
          (if (> (`self.Holding`) 0)
            (`GameplayStatics.PlaySound2D` "/Game/Sounds/Pickup_Sound_Cue.Pickup_Sound_Cue" 1.0 1.0 0.0 null null)
            ;;[1 1 1] Adding Holding to Rescued & adding to HUD
            (set `self.Rescued` (+ (`self.Rescued`) (`self.Holding`)))
            (set `self.Holding` 0)
            (bind _asmash_hud_2 (cast `/Game/Blueprints/Mash_HUD` (`PlayerController.GetHUD` (`GameplayStatics.GetPlayerController` 0))))))
        (:`CastFailed`
          ;;[1 1 1] If Hit Tree
          (cast `/Game/Blueprints/Tree` OtherActor)
          ;;[1 1 1] Play Game Over Effect and Stop Background Music
          (`GameplayStatics.PlaySound2D` "/Game/Sounds/Game_Over_Sound_Cue.Game_Over_Sound_Cue" 1.0 1.0 0.0 null null)
          (`AudioComponent.Stop` (`self.Background_Music`))
          ;;[1 1 1] Bring up Game-Over Screen
          (`GameplayStatics.SetGamePaused` true)
          (set `PlayerController.bShowMouseCursor` true (`GameplayStatics.GetPlayerController` 0))
          (bind _returnvalue (`|CreateWidget` "/Game/Blueprints/GameOver_Widget.GameOver_Widget_C"))
          (`UserWidget.AddToViewport` _returnvalue 0))))))

(event `InputAction|Reset`
  (params (Key :type "Key Structure"))
  ;[1 1 1] Press 'R' to Reset Level at anytime
  (:`Pressed`
    ;;[1 1 1] Destroy all actors, reset level and Load Level Again (Reset)
    (`KismetSystemLibrary.PrintString` "Reset!")
    (`self.K2_DestroyActor`)
    (bind _returnvalue (`GameplayStatics.GetCurrentLevelName` true))
    (`GameModeBase.ResetLevel` (`GameplayStatics.GetGameMode`))
    (`|ExecutionSequence`
      (:`then_0`
        (bind _outactors (`GameplayStatics.GetAllActorsOfClass` "/Game/Blueprints/SoldierCharacter.SoldierCharacter_C"))
        (`self.K2_DestroyActor` _outactors))
      (:`then_1`
        (bind _outactors_2 (`GameplayStatics.GetAllActorsOfClass` "/Game/Blueprints/Tree.Tree_C"))
        (`self.K2_DestroyActor` _outactors_2))
      (:`then_2`
        (bind _outactors_3 (`GameplayStatics.GetAllActorsOfClass` "/Game/Blueprints/Hospital.Hospital_C"))
        (`self.K2_DestroyActor` _outactors_3)
        (`LevelStreamingDynamic.LoadLevelInstance` _returnvalue (0.0 0.0 0.0) (struct) "" null)))))

(fn `Calculate Score`
  (set `self.Score` (* (+ (* (`self.Rescued`) 50) (* (`self.Holding`) 5)) (+ (* (`self.Seconds`) 25) (* (`self.Minutes`) 25)))))

(fn `UserConstructionScript`)