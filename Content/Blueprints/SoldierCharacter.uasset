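; Soldier character Blueprint that wanders between random nearby points and destroys itself when its render component leaves a hard-coded X/Y world boundary.
; GetNewLocation picks a random point at fixed height around a given centre, first the spawn location, then each reached target.
; Tick checks bounds and arrival, otherwise calls MoveComponentTo on the render component with a longer duration for distant targets, passing the world-space target as relative location.
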(event `self.ReceiveBeginPlay`
  (bind _output_get (set `self.Spawn Location` (`self.K2_GetActorLocation`)))
  (bind _returnvalue (`self.Get New Location` _output_get))
  (set `self.New Location` _returnvalue))

(event `self.ReceiveTick`
  (params (DeltaSeconds :type "Float (single-precision)"))
  (if (or (> (`.Y` (`KismetMathLibrary.BreakVector3f` (`SceneComponent.K2_GetComponentLocation` (`self.RenderComponent`)))) 82.0) (< (`.Y` (`KismetMathLibrary.BreakVector3f` (`SceneComponent.K2_GetComponentLocation` (`self.RenderComponent`)))) -95.0) (< (`KismetMathLibrary.BreakVector3f` (`SceneComponent.K2_GetComponentLocation` (`self.RenderComponent`))) -50.0) (> (`KismetMathLibrary.BreakVector3f` (`SceneComponent.K2_GetComponentLocation` (`self.RenderComponent`))) 135.0))
    ;[1 1 1] Character Movement Logic
    (`self.K2_DestroyActor`)
    (elif (== (`self.K2_GetActorLocation`) (`self.New Location`) :`ErrorTolerance` 0.5)
      (bind _returnvalue (`self.Get New Location` (`self.K2_GetActorLocation`)))
      (set `self.New Location` _returnvalue)
      (elif (> (`KismetMathLibrary.Vector_Distance` (`self.K2_GetActorLocation`) (`self.New Location`)) 30.0)
        (`KismetSystemLibrary.MoveComponentTo` (`self.RenderComponent`) (`self.New Location`) (`self.K2_GetActorRotation`) false false 3.0)
        (else
          (`KismetSystemLibrary.MoveComponentTo` (`self.RenderComponent`) (`self.New Location`) (`self.K2_GetActorRotation`) false false 1.0))))))

(fn `Get New Location`
  (params (InVec :type "Vector Structure"))
  (returns (ReturnValue :type "Vector Structure"))
  (bind _x (.x InVec))
  (bind _y (.y InVec))
  (return (`KismetMathLibrary.MakeVector` (`KismetMathLibrary.RandomFloatInRange` (- _x 10.0) (+ _x 10.0)) (`KismetMathLibrary.RandomFloatInRange` (- _y 5.0) (+ _y 5.0)) 15.0)))

(fn `UserConstructionScript`)