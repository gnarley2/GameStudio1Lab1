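; MashGameMode is a game mode that keeps the level populated with SoldierCharacter actors up to a maximum count.
; BeginPlay fills the population in a loop, then Tick recounts live soldiers and uses a Delay to throttle replacement spawns.
; Both paths use GetRandomSpawnLocation, which randomizes X and Y from scaled SpawnCentreLocation components (Y uses its Z) at fixed height, rotation and scale.
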(event `self.ReceiveBeginPlay`
  ;[1 1 1] Initial soldier population
  (set `self.Number Of Soldiers` 0)
  (`self.InitialSoldierSpawn`))

(event `self.ReceiveTick`
  (params (DeltaSeconds :type "Float (single-precision)"))
  ;[1 1 1] Checking how many Soldiers up to a max number, incorporates a delay then calls Spawn In Soldier Function
  (bind _outactors (`GameplayStatics.GetAllActorsOfClass` "/Game/Blueprints/SoldierCharacter.SoldierCharacter_C"))
  (bind _output_get (set `self.Number Of Soldiers` (`KismetArrayLibrary.Array_Length` _outactors)))
  (if (< _output_get (`self.Max Number Of Soldiers`))
    (`KismetSystemLibrary.Delay` 1.2)
    (`self.Spawn in Soldiers`)))

(fn `GetRandomSpawnLocation`
  (returns (`Random Location` :type "Transform Structure"))
  (bind _x (.x (`self.SpawnCentreLocation`)))
  (bind _z (.z (`self.SpawnCentreLocation`)))
  (return (`KismetMathLibrary.MakeTransform` (`KismetMathLibrary.MakeVector` (`KismetMathLibrary.RandomFloatInRange` (* _x -0.5) (* _x 2.5)) (`KismetMathLibrary.RandomFloatInRange` (* _z -5.0) (* _z 5.0)) 15.0) (struct :`Roll` -90.0) (0.25 0.25 0.25))))

(fn `InitialSoldierSpawn`
  (for _ (range (+ (`self.Number Of Soldiers`) 1) (+ (`self.Max Number Of Soldiers`) 1))
    (bind _random_location (`self.GetRandomSpawnLocation`))
    (`|SpawnActorFromClass` "/Game/Blueprints/SoldierCharacter.SoldierCharacter_C" _random_location "AdjustIfPossibleButDontSpawnIfColliding" "MultiplyWithRoot" null null)))

(fn `Spawn in Soldiers`
  ;[1 1 1] Additional check if should Spawn
  (if (!= (`self.Number Of Soldiers`) (`self.Max Number Of Soldiers`))
    (bind _random_location (`self.GetRandomSpawnLocation`))
    (`|SpawnActorFromClass` "/Game/Blueprints/SoldierCharacter.SoldierCharacter_C" _random_location "AdjustIfPossibleButDontSpawnIfColliding" "MultiplyWithRoot" null null)))

(fn `UserConstructionScript`)